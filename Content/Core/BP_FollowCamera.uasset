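; BP_FollowCamera is a camera actor that trails the first player's pawn at a configurable offset.
; Each Tick it interpolates its location toward the pawn's position plus Offset, axis by axis, without changing rotation.
; X uses CameraFollowSpeed with frame delta time, while Y and Z share CameraLateralInterpSpeed with a fixed time step, making their smoothing frame-rate dependent.
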(event `self.ReceiveTick`
  (params (DeltaSeconds :type "Float (single-precision)"))
  (bind _cameralateralinterpspeed (`self.CameraLateralInterpSpeed`))
  (`self.K2_SetActorLocation` (`KismetMathLibrary.MakeVector` (`KismetMathLibrary.FInterpTo` (.x (`self.K2_GetActorLocation`)) (.x (+ (`self.Offset`) (`self.K2_GetActorLocation` (`GameplayStatics.GetPlayerPawn` 0)))) DeltaSeconds (`self.CameraFollowSpeed`)) (`KismetMathLibrary.FInterpTo` (.y (`self.K2_GetActorLocation`)) (.y (+ (`self.Offset`) (`self.K2_GetActorLocation` (`GameplayStatics.GetPlayerPawn` 0)))) 0.03 _cameralateralinterpspeed) (`KismetMathLibrary.FInterpTo` (.z (`self.K2_GetActorLocation`)) (.z (+ (`self.Offset`) (`self.K2_GetActorLocation` (`GameplayStatics.GetPlayerPawn` 0)))) 0.03 _cameralateralinterpspeed))))

(fn `UserConstructionScript`)
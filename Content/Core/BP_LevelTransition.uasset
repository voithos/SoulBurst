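; BP_LevelTransition is an actor that fades the screen in at level start and out before restarting the level.
; The construction script creates a dynamic instance of M_LevelTransition and assigns it as a post process blendable.
; Fade timelines drive that material's "t" parameter, and the fade-out ends with a RestartLevel console command.
; The Restart input triggers the fade-out only when the Player is dead, while BeginFadeOut is an empty function.
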(event `self.ReceiveBeginPlay`
  (bind (_direction _t) (`Timeline|FadeIn`)
    (:`Update`
      (`MaterialInstanceDynamic.SetScalarParameterValue` (`self.TransitionMaterial`) "t" _t))))

(event `FadeOut`
  (bind (_direction _t) (`Timeline|FadeOutTimeline`)
    (:`Update`
      (`MaterialInstanceDynamic.SetScalarParameterValue` (`self.TransitionMaterial`) "t" _t))
    (:`Finished`
      (`KismetSystemLibrary.ExecuteConsoleCommand` "RestartLevel" null))))

(event `InputAction|Restart`
  (params (Key :type "Key Structure"))
  (:`Pressed`
    (bind _returnvalue (`GameplayStatics.GetActorOfClass` "/Game/Core/Player.Player_C"))
    (if (`/Game/Core/Player.IsDead` _returnvalue)
      (`self.FadeOut`))))

(fn `BeginFadeOut`)

(fn `UserConstructionScript`
  (bind _returnvalue (`KismetMaterialLibrary.CreateDynamicMaterialInstance` "/Game/Core/M_LevelTransition.M_LevelTransition"))
  (bind _output_get (set `self.TransitionMaterial` _returnvalue))
  (set `PostProcessComponent.Settings` (make `PostProcessSettings` :`WeightedBlendables` (make `WeightedBlendables` (`|MakeArray` (make `WeightedBlendable` 1.0 _output_get)))) (`self.PostProcess`)))